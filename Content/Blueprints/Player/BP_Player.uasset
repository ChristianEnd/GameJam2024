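; Player ship character that moves and fires through Enhanced Input, tracking health and score.
; A gate-and-delay loop repeats shots at a clamped fire rate, alternating muzzles or firing spread patterns.
; Interface events temporarily change bullet speed, spread and projectile type, add health, and report score to GM_InGame for level determination.
; HealthCheck handles death with an explosion, hidden meshes and a switch to StartTestMap.
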(event `self.ReceiveTick`
  (params (DeltaSeconds :type "Float (single-precision)")))

(event `/Game/Blueprints/Interfaces/BPI_Player.SetBulletSpeed`
  (params (BulletSpeed :type "Float (double-precision)") (BulletSpeedResetTime :type "Float (double-precision)"))
  ;[0.9492 0.324 1] InterfaceActions
  ;;[1 1 1] SetBulletSpeed
  (set `self.Projectile Speed` BulletSpeed)
  (`KismetSystemLibrary.Delay` BulletSpeedResetTime)
  (set `self.Projectile Speed` 3000.0))

(event `SetupInput`
  ;[0.5131 0.5994 1] SetupInput
  (bind _asplayer_controller (cast `PlayerController` (`self.GetController`)))
  (`/Engine/EditorBlueprintResources/StandardMacros.IsValid` _asplayer_controller
    (:`Is Valid`
      (`EnhancedInputSubsystemInterface.AddMappingContext` (pcsubsystem `EnhancedInputLocalPlayerSubsystem` _asplayer_controller) "/Game/Blueprints/Player/IMC_Player.IMC_Player" 0 (struct)))))

(event `self.ReceiveBeginPlay`
  ;[1 0.2341 0.3259] Start
  (`self.SetupInput`)
  (`self.SetPlayerStartVariables`))

(event `/Game/Blueprints/Interfaces/BPI_Player.SetSpray`
  (params (SprayInt :type Integer) (SprayDuration :type "Float (double-precision)"))
  ;[0.9492 0.324 1] InterfaceActions
  ;;[1 1 1] SetBulletSpray
  (set `self.BulletSpread` SprayInt)
  (`KismetSystemLibrary.RetriggerableDelay` SprayDuration)
  (set `self.BulletSpread` 1))

(event `SetPlayerStartVariables`
  ;[1 0.2341 0.3259] Start
  (`self.K2_SetActorLocation` (0.0 0.0 0.0))
  (set `CharacterMovementComponent.MaxWalkSpeed` (`self.Speed`) (`self.CharacterMovement`))
  (set `self.ProjectileStockSpeed` (`self.Projectile Speed`)))

(event `/Game/Blueprints/Interfaces/BPI_Player.AddHealth`
  (params (HealAmount :type "Float (double-precision)"))
  ;[0.9492 0.324 1] InterfaceActions
  ;;[1 1 1] Heal
  (set `self.Health` (+ HealAmount (`self.Health`))))

(event `/Game/Blueprints/Interfaces/BPI_Player.AddScore`
  (params (AddedScore :type Integer))
  ;[0.9492 0.324 1] InterfaceActions
  ;;[1 1 1] AddScore
  (`self.ScoreHandle` AddedScore)
  ;[0.4356 1 0.9806] SetScoreInGameModeToDetermineLevel
  (bind _asgm_in_game (cast `/Game/Blueprints/Essential/GM_InGame` (`GameplayStatics.GetGameMode`)))
  (if (< (`self.ActualScore`) 0)
    (set `self.ActualScore` 0))
  (`/Game/Blueprints/Essential/GM_InGame.SetPlayerScore` _asgm_in_game (`self.ActualScore`) (`KismetMathLibrary.Round` (`self.Health`))))

(event `EnhancedInput|/Game/Blueprints/Player/Actions/IA_Move`
  (params (ActionValue :type "Vector2D Structure") (ElapsedSeconds :type "Float (double-precision)") (TriggeredSeconds :type "Float (double-precision)") (InputAction :type "InputAction Object Reference" :default "/Game/Blueprints/Player/Actions/IA_Move.IA_Move"))
  (bind _returnvalue_roll (`KismetMathLibrary.BreakRotator` (`self.GetControlRotation`)))
  (bind (_returnvalue_roll_2 _returnvalue_pitch) (`KismetMathLibrary.BreakRotator` (`self.GetControlRotation`)))
  ;[0.5107 0.7539 1] MovementInput
  (:`Triggered`
    (`self.AddMovementInput` (`KismetMathLibrary.GetRightVector` (`KismetMathLibrary.MakeRotator` _returnvalue_roll)) ActionValue_X)
    (`self.AddMovementInput` (`KismetMathLibrary.GetForwardVector` (`KismetMathLibrary.MakeRotator` 0.0 _returnvalue_pitch)) ActionValue_Y)))

(event `/Game/Blueprints/Interfaces/BPI_Player.BulletType`
  (params (BulletInArray :type Integer) (TimeToSwitchBack :type "Float (double-precision)"))
  ;[0.9492 0.324 1] InterfaceActions
  ;;[1 1 1] SetProjectileType
  (set `self.ActiveProjectile` (`|GetArrayItem` (`self.ProjectileArrayPlayer`) BulletInArray))
  (`KismetSystemLibrary.Delay` TimeToSwitchBack)
  (set `self.ActiveProjectile` (`|GetArrayItem` (`self.ProjectileArrayPlayer`))))

(event `ForceFiring`
  (bind _projectile_speed (`self.Projectile Speed`))
  (bind _projectile_speed_2 (`self.Projectile Speed`))
  (if (not (`self.LockFiring`)) :!label _label
    (if (`self.CanFire`)
      (`|ExecutionSequence`
        (:`then_0`
          (goto _label_2 :!via `Open`))
        (:`then_1`
          (`/Engine/EditorBlueprintResources/StandardMacros.Gate` true :!label _label_2
            (:`Exit`
              (`|ExecutionSequence`
                (:`then_0`
                  _)
                (:`then_1`
                  (`KismetSystemLibrary.Delay` (`KismetMathLibrary.FClamp` (* (`self.FireRate`) (`self.FireRateMulti`)) 0.03) :!label _label_3)
                  (set `self.CanFire` true)
                  (goto _label_2)))))))
      (else
        (`|ExecutionSequence`
          (:`then_0`
            (goto _label_2 :!via `Open`))
          (:`then_1`
            (goto _label_3)))))
    (if (`self.FireFlipFlop`)
      (`/Engine/EditorBlueprintResources/StandardMacros.FlipFlop`
        (:`A`
          (`|SpawnActorFromClass` (`self.ActiveProjectile`) (`KismetMathLibrary.MakeTransform` (`SceneComponent.K2_GetComponentLocation` (`self.ShipTestBody01`)) (`self.BulletRotation`)) "Undefined" "MultiplyWithRoot" null (`self.DamageMulti`) 10000.0 null))
        (:`B`
          (`|SpawnActorFromClass` (`self.ActiveProjectile`) (`KismetMathLibrary.MakeTransform` (`SceneComponent.K2_GetComponentLocation` (`self.ShipTestBody02`)) (`self.BulletRotation`)) "Undefined" "MultiplyWithRoot" null (`self.DamageMulti`) 10000.0 null)))
      (else
        (switch `int` (`self.BulletSpread`)
          (:`0`
            (`|SpawnActorFromClass` (`self.ActiveProjectile`) (`KismetMathLibrary.MakeTransform` (`SceneComponent.K2_GetComponentLocation` (`self.BulletSpawnPoint01`)) (`self.BulletRotation`)) "Undefined" "MultiplyWithRoot" null (`self.DamageMulti`) (`self.Projectile Speed`) null))
          (:`1`
            (`|SpawnActorFromClass` (`self.ActiveProjectile`) (`KismetMathLibrary.MakeTransform` (`SceneComponent.K2_GetComponentLocation` (`self.BulletSpawnPoint02`)) (`self.BulletRotation`)) "Undefined" "MultiplyWithRoot" null (`self.DamageMulti`) _projectile_speed_2 null)
            (`|SpawnActorFromClass` (`self.ActiveProjectile`) (`KismetMathLibrary.MakeTransform` (`SceneComponent.K2_GetComponentLocation` (`self.BulletSpawnPoint03`)) (`self.BulletRotation`)) "Undefined" "MultiplyWithRoot" null (`self.DamageMulti`) _projectile_speed_2 null))
          (:`2`
            (`|SpawnActorFromClass` (`self.ActiveProjectile`) (`KismetMathLibrary.MakeTransform` (`SceneComponent.K2_GetComponentLocation` (`self.BulletSpawnPoint01`)) (`self.BulletRotation`)) "Undefined" "MultiplyWithRoot" null (`self.DamageMulti`) _projectile_speed null)
            (`|SpawnActorFromClass` (`self.ActiveProjectile`) (`KismetMathLibrary.MakeTransform` (`SceneComponent.K2_GetComponentLocation` (`self.BulletSpawnPoint02`)) (`self.BulletRotation`)) "Undefined" "MultiplyWithRoot" null (`self.DamageMulti`) _projectile_speed null)
            (`|SpawnActorFromClass` (`self.ActiveProjectile`) (`KismetMathLibrary.MakeTransform` (`SceneComponent.K2_GetComponentLocation` (`self.BulletSpawnPoint03`)) (`self.BulletRotation`)) "Undefined" "MultiplyWithRoot" null (`self.DamageMulti`) _projectile_speed null)))))
    (set `self.CanFire` false)))

(event `EnhancedInput|/Game/Blueprints/Player/Actions/IA_Shoot`
  (params (ActionValue :type Boolean) (ElapsedSeconds :type "Float (double-precision)") (TriggeredSeconds :type "Float (double-precision)") (InputAction :type "InputAction Object Reference" :default "/Game/Blueprints/Player/Actions/IA_Shoot.IA_Shoot"))
  (:`Started`
    (if (`self.Alive`)
      (goto _label)))
  (:`Completed`
    (if (not (`self.LockFiring`))
      (goto _label_2 :!via `Close`))))

(event `StopFiring`
  (params (LockFiring :type Boolean))
  (if LockFiring
    (set `self.LockFiring` true)
    (goto _label_2 :!via `Close`)))

(fn `HealthCheck`
  (if (<= (`self.Health`) 0.0)
    (set `self.Alive` false)
    (`GameplayStatics.SpawnEmitterAtLocation` "/Game/StarterContent/Particles/P_Explosion.P_Explosion" (`self.K2_GetActorLocation`) (struct) (3.0 3.0 3.0))
    (`SceneComponent.SetVisibility` (`self.Mesh`) false false)
    (`SceneComponent.SetVisibility` (`self.ShipTestBody`) false false)
    (`SceneComponent.SetVisibility` (`self.ShipTestBody01`) false false)
    (`SceneComponent.SetVisibility` (`self.ShipTestBody02`) false false)
    (`SceneComponent.SetVisibility` (`self.ShipTestBody03`) false false)
    (`GameplayStatics.OpenLevel` "StartTestMap")))

(fn `ScoreHandle`
  (params (AddedScore :type Integer))
  (set `self.ActualScore` (+ AddedScore (`self.ActualScore`))))

(fn `UserConstructionScript`)