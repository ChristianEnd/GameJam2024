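; Parent pickup actor that grants either a spray pattern or health to players overlapping its sphere.
; On overlap, it checks for BPI_Player, then the HealtOrBullets flag selects SetSpray (true) or AddHealth (false).
; The construction script applies a configurable mesh.
; Tick adds a velocity-scaled X offset, then negates the entire position, flipping the actor across the world origin each frame.
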(event `self.ReceiveTick`
  (params (DeltaSeconds :type "Float (single-precision)"))
  (`self.K2_SetActorLocation` (* (+ (`self.K2_GetActorLocation`) (`KismetMathLibrary.MakeVector` (* DeltaSeconds (`self.Velocity`)))) -1.0)))

(event `self.Sphere.OnComponentBeginOverlap`
  (params (OverlappedComponent :type "PrimitiveComponent Object Reference") (OtherActor :type "Actor Object Reference") (OtherComp :type "PrimitiveComponent Object Reference") (OtherBodyIndex :type Integer) (bFromSweep :type Boolean) (SweepResult :type "HitResult Structure (by ref)"))
  (if (`KismetSystemLibrary.DoesImplementInterface` OtherActor "/Game/Blueprints/Interfaces/BPI_Player.BPI_Player_C")
    (if (`self.HealtOrBullets`)
      (bind _asbpi_player (cast `/Game/Blueprints/Interfaces/BPI_Player` OtherActor))
      (`/Game/Blueprints/Interfaces/BPI_Player.SetSpray` _asbpi_player (`self.SprayPattern`))
      (else
        (bind _asbpi_player_2 (cast `/Game/Blueprints/Interfaces/BPI_Player` OtherActor))
        (`/Game/Blueprints/Interfaces/BPI_Player.AddHealth` _asbpi_player_2 (`self.Heal Amount`))))))

(fn `UserConstructionScript`
  (`StaticMeshComponent.SetStaticMesh` (`self.Mesh`) (`self.New Mesh`)))