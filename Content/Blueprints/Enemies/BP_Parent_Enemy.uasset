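; Base enemy character that advances at a set walk speed against its control-rotation forward vector, shoots, and rewards the player on death.
; When CanShoot is set, a gate-and-delay loop spawns projectiles within a world X band at the FireRate interval.
; The same flag starts two timelines that sway the capsule via local X/Y offsets.
; HealthCheck handles death with an explosion, score through BPI_Player, a random pickup for scoring enemies, and destruction.
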(event `self.ReceiveBeginPlay`
  (bind _forwardvelocity (`self.ForwardVelocity`))
  (bind _charactermovement (`self.CharacterMovement`))
  (set `CharacterMovementComponent.MaxWalkSpeed` _forwardvelocity _charactermovement)
  (set `CharacterMovementComponent.MaxWalkSpeedCrouched` _forwardvelocity _charactermovement)
  (bind _asbpi_player (cast `/Game/Blueprints/Interfaces/BPI_Player` (`GameplayStatics.GetPlayerPawn` 0)))
  (set `self.As BPI Player` _asbpi_player)
  (set `self.RelativeStartLocation` (`SceneComponent.RelativeLocation` (`self.CapsuleComponent`)))
  (if (`self.CanShoot`)
    (`self.StartFire`)
    (`self.SwizzleEnemyMovement`)))

(event `self.ReceiveTick`
  (params (DeltaSeconds :type "Float (single-precision)"))
  (`self.AddMovementInput` (`KismetMathLibrary.GetForwardVector` (`self.GetControlRotation`)) -1.0)
  (`TimelineComponent.SetPlayRate` (`self.TL_SwizzleMovement X`) (`self.PlayRateMovementXAxis`))
  (`TimelineComponent.SetPlayRate` (`self.TL_SwizzleMovement Y`) (`self.PlayRateMovementYAxis`)))

(event `StartFire`
  (bind _returnvalue_x (`KismetMathLibrary.BreakVector` (`self.K2_GetActorLocation`)))
  (`|ExecutionSequence`
    (:`then_0`
      (goto _label :!via `Open`))
    (:`then_1`
      (`/Engine/EditorBlueprintResources/StandardMacros.Gate` true :!label _label
        (:`Exit`
          (`|ExecutionSequence`
            (:`then_0`
              (if (`KismetMathLibrary.InRange_FloatFloat` _returnvalue_x -2000.0 13000.0)
                (`|SpawnActorFromClass` (`self.ProjectileParent`) (`KismetMathLibrary.MakeTransform` (`SceneComponent.K2_GetComponentLocation` (`self.FireLocation`)) (`self.ShootRotationMid`)) "Undefined" "MultiplyWithRoot" null 1.0 3000.0 null)))
            (:`then_1`
              (`KismetSystemLibrary.Delay` (* 1.0 (`self.FireRate`)))
              (goto _label))))))))

(event `DestroyActor`
  (`KismetSystemLibrary.RetriggerableDelay` 0.1)
  (`self.K2_DestroyActor`))

(event `SwizzleEnemyMovement`
  (bind _ymulti (`self.YMulti`))
  (bind _xmulti (`self.XMulti`))
  (`KismetSystemLibrary.Delay` 0.2)
  (`|ExecutionSequence`
    (:`then_0`
      (bind (_direction _newtrack_0) (`Timeline|TL_SwizzleMovement X` :!via `PlayFromStart`)
        (:`Update`
          (`SceneComponent.K2_AddLocalOffset` (`self.CapsuleComponent`) (`KismetMathLibrary.MakeVector` (`KismetMathLibrary.Lerp` (* _xmulti -1.0) _xmulti _newtrack_0)) false false))))
    (:`then_1`
      (bind (_direction_2 _newtrack_0_2) (`Timeline|TL_SwizzleMovement Y` :!via `PlayFromStart`)
        (:`Update`
          (`SceneComponent.K2_AddLocalOffset` (`self.CapsuleComponent`) (`KismetMathLibrary.MakeVector` 0.0 (`KismetMathLibrary.Lerp` (* _ymulti -1.0) _ymulti _newtrack_0_2)) false false))))))

(fn `HealthCheck`
  (bind _returnvalue (`self.GetTransform`))
  (bind _scoregivebase (`self.ScoreGiveBase`))
  (bind _pickuparray (`self.PickUpArray`))
  (if (<= (`self.Health`) 0.0)
    (`GameplayStatics.SpawnEmitterAtLocation` "/Game/StarterContent/Particles/P_Explosion.P_Explosion" (`self.K2_GetActorLocation`) (struct) (5.0 5.0 5.0))
    (`/Game/Blueprints/Interfaces/BPI_Player.AddScore` (`self.As BPI Player`) _scoregivebase)
    (if (> _scoregivebase 0)
      (`|SpawnActorFromClass` (`|GetArrayItem` _pickuparray (`KismetMathLibrary.RandomIntegerInRange` 0 (- (`KismetArrayLibrary.Array_Length` _pickuparray) 1))) (`KismetMathLibrary.MakeTransform` (`KismetMathLibrary.MakeVector` (.x (.location _returnvalue)) (.y (.location _returnvalue))) (.rotation _returnvalue)) "Undefined" "MultiplyWithRoot" null 1200.0 null))
    (`self.DestroyActor`)))

(fn `UserConstructionScript`
  (bind _charactermovement (`self.CharacterMovement`))
  (bind _output_get (set `CharacterMovementComponent.MaxWalkSpeed` (`self.ForwardVelocity`) _charactermovement))
  (set `CharacterMovementComponent.MaxWalkSpeedCrouched` _output_get _charactermovement))