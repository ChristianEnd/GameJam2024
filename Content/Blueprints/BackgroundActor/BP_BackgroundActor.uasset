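; BP_BackgroundActor is a background mesh actor that moves steadily along negative X.
; The construction script applies a configurable mesh, and BeginPlay records the starting location.
; Tick shifts X by Speed scaled by delta time, passing the world location into SetActorRelativeLocation.
; ResetPosition teleports the actor back to its stored start, with no call to it inside this Blueprint.
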(event `self.ReceiveBeginPlay`
  (set `self.StartLocation` (`self.K2_GetActorLocation`)))

(event `/Game/Blueprints/Interfaces/BPI_BackgroundObjects.ResetPosition`
  (`self.K2_SetActorLocation` (`self.StartLocation`) false true))

(event `self.ReceiveTick`
  (params (DeltaSeconds :type "Float (single-precision)"))
  (bind (_actuallocation_x _actuallocation_y _actuallocation_z) (`KismetMathLibrary.BreakVector` (`self.ActualLocation`)))
  (set `self.ActualLocation` (`self.K2_GetActorLocation`))
  (`self.K2_SetActorRelativeLocation` (`KismetMathLibrary.MakeVector` (- _actuallocation_x (* DeltaSeconds (`self.Speed`))) _actuallocation_y _actuallocation_z)))

(fn `UserConstructionScript`
  (`StaticMeshComponent.SetStaticMesh` (`self.Mesh`) (`self.NewMesh`)))